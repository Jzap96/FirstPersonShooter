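; Enemy AI character that stays still until Pawn Sensing sees a pawn, then moves toward the player with AI MoveTo.
; Each move request plays a gated montage as the attack, but applies no damage to the player.
; Projectile overlaps on its sphere apply self-damage and play an impact sound.
; Damage updates the health widget, and at zero health the enemy spawns an emitter and is destroyed.
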(event `self.ReceiveBeginPlay`
  ;[1 1 1] Enemy Health
  (bind _asenemy_health (cast `/Game/EnemyHealth/EnemyHealth` (`WidgetComponent.GetUserWidgetObject` (`self.Widget`))))
  (bind _output_get (set `self.As Enemy Health` _asenemy_health))
  (set `/Game/EnemyHealth/EnemyHealth.CurrentHealt` (`self.CurrentHealth`) _output_get)
  (set `/Game/EnemyHealth/EnemyHealth.MaxHealth` (`self.MaxHealth`) _output_get))

(event `self.ReceiveTick`
  (params (DeltaSeconds :type "Float (single-precision)"))
  ;[1 1 1] Navigation
  (if (not (`self.playerOnSight`))
    (`MovementComponent.StopMovementImmediately` (`self.CharacterMovement`))))

(event `self.PawnSensing.OnSeePawn`
  (params (Pawn :type "Pawn Object Reference"))
  ;[1 1 1] Navigation
  (set `self.playerOnSight` true)
  (`self.FollowPlayer`))

(event `FollowPlayer`
  ;[1 1 1] Navigation
  (if (`self.playerOnSight`)
    (set `self.canAttack` true)
    (`|AIMoveTo` self (0.0 0.0 0.0) (`GameplayStatics.GetPlayerCharacter` 0) 70.0
      (:`then`
        (if (`self.canAttack`)
          (set `self.canAttack` false)
          (bind _returnvalue (`self.PlayAnimMontage` null))
          (`KismetSystemLibrary.Delay` _returnvalue)
          (set `self.canAttack` true))))
    (else
      (set `self.playerOnSight` false))))

(event `Attack`
  ;[1 1 1] Navigation
)

(event `self.Sphere.OnComponentBeginOverlap`
  (params (OverlappedComponent :type "PrimitiveComponent Object Reference") (OtherActor :type "Actor Object Reference") (OtherComp :type "PrimitiveComponent Object Reference") (OtherBodyIndex :type Integer) (bFromSweep :type Boolean) (SweepResult :type "HitResult Structure (by ref)"))
  ;[1 1 1] Appyl Damage
  (cast `/Game/FPS_Level/Blueprints/BP_FirstPersonProjectile` OtherActor)
  (`GameplayStatics.ApplyDamage` self 0.25)
  (`GameplayStatics.PlaySound2D` "/Game/SFX/Bullet_Impact__Sound_Effect.Bullet_Impact__Sound_Effect" 1.0 1.0 0.0 null null))

(event `self.ReceiveAnyDamage`
  (params (Damage :type "Float (single-precision)") (DamageType :type "DamageType Object Reference") (InstigatedBy :type "Controller Object Reference") (DamageCauser :type "Actor Object Reference"))
  (bind _output_get (set `self.CurrentHealth` (- (`self.CurrentHealth`) (* Damage 100.0))))
  (`/Game/EnemyHealth/EnemyHealth.Update HEalth` (`self.As Enemy Health`) _output_get)
  (if (<= (`self.CurrentHealth`) 0)
    (`GameplayStatics.SpawnEmitterAttached` null (`self.CapsuleComponent`))
    (`self.K2_DestroyActor`)))

(fn `UserConstructionScript`)